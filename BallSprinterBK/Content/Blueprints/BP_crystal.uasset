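; Crystal actor that flies into the player when touched, then disappears, with no reward or scoring logic in this graph.
; Overlap with the first player's pawn stores the crystal's location and plays the TL_Crystal_Move timeline.
; Each update lerps from that stored point to the pawn's current location by the timeline alpha, so it follows a moving player.
; The actor destroys itself when the timeline finishes.
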(event Collision|EventActorBeginOverlap
  (params (OtherActor :type Actor%20Object%20Reference))
  (if (== OtherActor (Game|Player|GetPlayerPawn 0))
    (bind _output_get (Variables|Default|SetLerpStartLocation (Transformation|GetActorLocation)))
    (bind _alphablend (Timeline|TL_Crystal_Move Play)
      (:Update
        (Transformation|SetActorLocation (Math|Vector|Lerp(Vector) _output_get (Transformation|GetActorLocation (Game|Player|GetPlayerPawn 0)) _alphablend) false false))
      (:Finished
        (Actor|DestroyActor)))))

(fn ConstructionScript)