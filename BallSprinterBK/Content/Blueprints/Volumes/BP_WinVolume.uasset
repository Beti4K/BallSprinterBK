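; BP_WinVolume is a level-exit volume that advances the player to the next level once no crystals remain.
; On player overlap, it searches the world for BP_crystal actors and prints a warning if any exist.
; Otherwise it finds the current level in the TabLevelnames array and opens the following entry, or quits the game on the last one.
; CompleteLevel is an empty stub.
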(event Collision|EventActorBeginOverlap
  (params (OtherActor :type Actor%20Object%20Reference))
  (Utilities|IsPlayer OtherActor
    (:IsPlayer
      (if (Pure|CheckAnyCrystals)
        (Development|PrintString "You don't have all crystals yet!")
        (else
          (Impure|LoadNextLevel))))))

(fn ConstructionScript)

(fn IsFinal
  (return (== (Pure|GetCurrentIndex) (Utilities|Array|LastIndex (Variables|Default|Gettab_levelnames)))))

(fn GetCurrentIndex
  (bind _returnvalue (Game|GetCurrentLevelName true))
  (return (Utilities|Array|FindItem (Variables|Default|Gettab_levelnames) (Utilities|String|StringToName _returnvalue))))

(fn CheckAnyCrystals
  (bind _outactors (Actor|GetAllActorsOfClass "/Game/Blueprints/Actors/BP_crystal.BP_crystal_C"))
  (return (> (Utilities|Array|Length _outactors) 0)))

(fn CompleteLevel)

(fn LoadNextLevel
  (if (Pure|IsFinal)
    (Game|QuitGame 0 "Quit" false)
    (else
      (Game|OpenLevel(byName) (Utilities|Array|Get(acopy) (Variables|Default|Gettab_levelnames) (+ (Pure|GetCurrentIndex) 1))))))