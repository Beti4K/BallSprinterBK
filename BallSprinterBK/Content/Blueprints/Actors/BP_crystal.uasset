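; BP_crystal is a collectible crystal that the player picks up by overlapping it.
; On overlap it caches its location, then a timeline lerps it toward the player pawn's live position while shrinking its scale and changing its point light intensity.
; When the timeline finishes it destroys itself and prints a completion message if no other BP_crystal actors remain.
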(event Collision|EventActorBeginOverlap
  (params (OtherActor :type Actor%20Object%20Reference))
  (Utilities|IsPlayer OtherActor
    (:IsPlayer
      (bind _output_get (CallFunction|CrystalCurrentPosition))
      (bind (_direction _alphablend _scale _lightchange) (Timeline|TL_Crystal_Move Play)
        (:Update
          (CallFunction|MoveCrystaltoPlayerPawn _output_get _alphablend)
          (CallFunction|ChangeCrystalScale _scale)
          (CallFunction|FlashingEffect _lightchange))
        (:Finished
          (Actor|DestroyActor)
          (CallFunction|CheckifAllCrystals))))))

(fn ConstructionScript)

(fn MoveCrystaltoPlayerPawn
  (params (A :type Vector) (Alpha :type Float%20%28single-precision%29))
  (Transformation|SetActorLocation (Math|Vector|Lerp(Vector) A (Transformation|GetActorLocation (Game|Player|GetPlayerPawn 0)) Alpha) false false))

(fn CrystalCurrentPosition
  (bind _output_get (Variables|Default|SetLerpStartLocation (Transformation|GetActorLocation)))
  (return _output_get))

(fn ChangeCrystalScale
  (params (Alpha :type Float%20%28single-precision%29))
  (Transformation|SetActorScale3D (Math|Vector|Lerp(Vector) (Transformation|GetActorScale3D) "0, 0, 0" Alpha)))

(fn FlashingEffect
  (params (Alpha :type Float%20%28single-precision%29))
  (Rendering|Components|Light|SetIntensity (Variables|Default|GetPointLight) (Math|Float|Lerp 5e+02 5e+03 Alpha)))

(fn CheckifAllCrystals
  (bind _outactors (Actor|GetAllActorsOfClass "BP_crystal_C"))
  (if (not (> (Utilities|Array|Length _outactors) 0))
    (Development|PrintString "You got them all!")))