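; Spike trap actor that periodically moves vertically and restarts the level when the player touches it.
; After each configurable delay, a timeline lerps its Z between absolute down and up heights, then loops back to the delay when finished.
; Player overlap starts a held camera fade-out, prints "OOF!" and reopens the current level after a brief delay.
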(event Collision|EventActorBeginOverlap
  (params (OtherActor :type Actor%20Object%20Reference))
  (Utilities|IsPlayer OtherActor
    (:IsPlayer
      (CameraFades|StartCameraFade :self (Game|GetPlayerCameraManager 0) :ToAlpha 1.0 :bHoldWhenFinished true)
      (Development|PrintString "OOF!" true false)
      (Utilities|FlowControl|Delay 0.1)
      (bind _returnvalue (Game|GetCurrentLevelName true))
      (Game|OpenLevel(byName) (Utilities|String|StringToName _returnvalue)))))

(event EventBeginPlay
  (bind _returnvalue (Transformation|GetActorLocation))
  (Utilities|FlowControl|Delay (Variables|SpikesOptions|GetDuration) :!label _label)
  (bind _spikesout (Timeline|Timeline_0 PlayFromStart)
    (:Update
      (Transformation|SetActorLocation (Math|Vector|Lerp(Vector) (Math|Vector|MakeVector (.x _returnvalue) (.y _returnvalue) (Variables|SpikesOptions|GetHowMuchDown)) (Math|Vector|MakeVector (.x _returnvalue) (.y _returnvalue) (Variables|SpikesOptions|GetHow%20Much%20Up)) _spikesout) false false))
    (:Finished
      (goto _label))))

(fn ConstructionScript)