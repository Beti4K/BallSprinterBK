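; Auto-firing cannon actor that repeatedly plays a recoil animation and spawns BP_ammo1 projectiles.
; From BeginPlay, a loop waits ShootingSpeed, then plays the TL_CannonShot timeline to slide the Cannon component along local Y.
; Separately, Tick drives a Delay of ShootingSpeed plus a fixed offset, spawning ammo at the Arrow's transform, scaled by AmmoScale.
; Recoil and spawning are timed independently, with no direct link between them.
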(event EventTick
  (params (DeltaSeconds :type Float%20%28single-precision%29))
  (bind _arrow (Variables|Default|GetArrow))
  (Utilities|FlowControl|Delay (+ (Variables|CannonProp|GetShootingSpeed) 0.5))
  (Game|SpawnActorfromClass "/Game/Blueprints/Actors/BP_ammo1.BP_ammo1_C" (Math|Transform|MakeTransform (Transformation|GetWorldLocation _arrow) (Transformation|GetWorldRotation _arrow) (Math|Conversions|ToVector(Float) (Variables|CannonProp|GetammoScale))) "Undefined" 0 0))

(event EventBeginPlay
  (Utilities|FlowControl|Delay (Variables|CannonProp|GetShootingSpeed) :!label _label)
  (bind _cannonrecoil (Timeline|TL_CannonShot PlayFromStart)
    (:Update
      (Transformation|SetRelativeLocation (Variables|Default|GetCannon) (Math|Vector|MakeVector 0.0 _cannonrecoil 0.0) false false))
    (:Finished
      (goto _label))))

(fn ConstructionScript)