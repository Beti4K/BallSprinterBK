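; BP_ammo1 is a hazardous ammo actor that restarts the current level when it overlaps the player pawn.
; Its overlap event branches to AmmoRestart for the player, which fades the camera out, prints a message, then reopens the level by name after a brief delay.
; Any other overlap runs AmmoDestroy, which removes the actor after a short delay.
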(event Collision|EventActorBeginOverlap
  (params (OtherActor :type Actor%20Object%20Reference))
  (if (== OtherActor (Game|Player|GetPlayerPawn 0))
    (Utilities|AmmoRestart)
    (else
      (Utilities|AmmoDestroy))))

(fn ConstructionScript)