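; Player pawn that moves by physics torque, with a rotatable spring-arm camera and a level restart on damage.
; The left-right axis adds scaled torque on both X and Y of the Player component, while the up-down axis is unwired.
; Q and E call the CameraRotation macro to step the spring arm's yaw either way by RotationModifier.
; Any damage runs Level_Restart, which fades the camera out, waits, then reopens the current level.
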(event Game|Damage|EventAnyDamage
  (params (Damage :type Float%20%28single-precision%29) (DamageType :type Damage%20Type%20Object%20Reference) (InstigatedBy :type Controller%20Object%20Reference) (DamageCauser :type Actor%20Object%20Reference))
  (Utilities|LevelRestart))

(event Input|AxisEvents|InputAxisleft-right
  (params (AxisValue :type Float%20%28single-precision%29))
  (bind _multiply (Variables|Default|GetMultiply))
  (Class|PrimitiveComponent|AddTorqueinRadians (Variables|Default|GetPlayer) (Math|Vector|MakeVector (* (stale Input|AxisEvents|InputAxisup-down AxisValue) _multiply) (* AxisValue _multiply) 0.0) "None" true))

(event Input|AxisEvents|InputAxisup-down
  (params (AxisValue :type Float%20%28single-precision%29)))

(event Input|KeyboardEvents|E
  (params (Key :type Key%20Structure :default "None"))
  (:Pressed
    (Utilities|CameraRotation) ; enters at RightIn
  ))

(event Input|KeyboardEvents|Q
  (params (Key :type Key%20Structure :default "None"))
  (:Pressed
    (bind _change (Utilities|CameraRotation))))

(fn ConstructionScript)